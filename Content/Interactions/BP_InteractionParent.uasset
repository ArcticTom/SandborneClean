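; Base interactable actor with a configurable mesh, sphere trigger and widget component that displays an interaction description.
; The construction script applies the mesh, trigger and UI settings from variables, and BeginPlay passes the description to the widget.
; Trigger overlaps add or remove the actor from the Character_BP's interactions.
; ToggleUI sets prompt visibility, while Interact stores the interacting character and only prints a debug string.
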(event OnComponentBeginOverlap(InteractionTrigger)
  (params (OverlappedComponent :type Primitive%20Component%20Object%20Reference) (OtherActor :type Actor%20Object%20Reference) (OtherComp :type Primitive%20Component%20Object%20Reference) (OtherBodyIndex :type Integer) (bFromSweep :type Boolean) (SweepResult :type Hit%20Result%20Structure%20%28by%20ref%29))
  ;[1 1 1] Player enters trigger radius
  (bind _ascharacter_bp (Utilities|Casting|CastToCharacter_BP OtherActor))
  (Default|AddInteraction _ascharacter_bp self))

(event OnComponentEndOverlap(InteractionTrigger)
  (params (OverlappedComponent :type Primitive%20Component%20Object%20Reference) (OtherActor :type Actor%20Object%20Reference) (OtherComp :type Primitive%20Component%20Object%20Reference) (OtherBodyIndex :type Integer))
  ;[1 1 1] Player enters trigger radius
  (bind _ascharacter_bp (Utilities|Casting|CastToCharacter_BP OtherActor))
  (Default|RemoveInteraction _ascharacter_bp self))

(event EventBeginPlay
  (bind _aswbp_interaction_ui (Utilities|Casting|CastToWBP_Interaction_UI (UserInterface|GetUserWidgetObject (Variables|Default|GetInteractionUI))))
  (bind _output_get (Variables|Default|SetInteractionUIWidget _aswbp_interaction_ui))
  (Default|SetInteractionDescription _output_get (Variables|Configuration|GetInteractDescription)))

(fn ConstructionScript
  (Configuration|SetupMesh)
  (Configuration|SetupTrigger)
  (Configuration|SetupUI))

(fn SetupMesh
  ;[1 1 1] Set static mesh and relative transform
  (Components|StaticMesh|SetStaticMesh (Variables|Default|GetInteractionMesh) (Variables|Configuration|GetInteractMesh))
  (Transformation|SetRelativeTransform (Variables|Default|GetInteractionMesh) (Variables|Configuration|GetMeshTransform) false false))

(fn SetupTrigger
  ;[1 1 1] Configure Trigger radius and location
  (Components|Sphere|SetSphereRadius (Variables|Default|GetInteractionTrigger) (Variables|Configuration|GetTriggerRadius) true)
  (Transformation|SetRelativeLocation (Variables|Default|GetInteractionTrigger) (Variables|Configuration|GetTriggerLocation) false false))

(fn SetupUI
  ;[1 1 1] Setup UI location offset - default hovers on top
  (Transformation|SetRelativeLocation (Variables|Default|GetInteractionUI) (Variables|Configuration|GetUILocation) false false))

(fn ToggleUI
  (params (Visibile :type Boolean))
  (Rendering|SetVisibility (Variables|Default|GetInteractionUI) Visibile false))

(fn Interact
  (params (InteractingCharacter :type Character%20BP%20Object%20Reference))
  (Variables|Default|SetInteractCharacter InteractingCharacter)
  (Development|PrintString "Interacting"))