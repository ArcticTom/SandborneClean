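; Interactable switch that toggles between on and off each time a character interacts with it, building on a parent interaction Blueprint.
; Interact runs the parent logic, flips the Active flag and swaps the interaction mesh's material to match.
; When the interaction UI widget is valid, it updates the Turn On/Turn Off prompt and calls Activate or Deactivate, so those calls are skipped without a widget.
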(event EventInteract
  (params (InteractingCharacter :type Character%20BP%20Object%20Reference))
  (bind _interactionmesh (Variables|Default|GetInteractionMesh))
  (|CallParentFunction InteractingCharacter)
  (if (not (Variables|Default|GetbActive))
    (Variables|Default|SetbActive true) ; Not currently active, switch on
    (Rendering|Material|SetMaterial _interactionmesh 0 "/Game/Mannequin/Character/Materials/M_UE4Man_ChestLogo.M_UE4Man_ChestLogo")
    (bind _interactionuiwidget (Variables|Default|GetInteractionUIWidget)
      (:then
        (Default|SetInteractionDescription _interactionuiwidget "Turn Off")
        (Default|CallActivate))
      (:else))
    (else
      (Variables|Default|SetbActive false)
      (Rendering|Material|SetMaterial _interactionmesh 0 "/Game/Geometry/Meshes/CubeMaterial.CubeMaterial")
      (bind _interactionuiwidget_2 (Variables|Default|GetInteractionUIWidget)
        (:then
          (Default|SetInteractionDescription _interactionuiwidget_2 "Turn On")
          (Default|CallDeactivate))
        (:else)))))

(fn ConstructionScript
  (|CallParentFunction))